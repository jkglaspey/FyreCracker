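; BP_LinearAI is an AI character that wanders the map and shoots at other BP_LinearAI pawns it spots.
; BeginControllingCharacter, not triggered here, waits for landing, then starts SearchAround, a self-repeating random-point move that also waits out falls on failure.
; Pawn sensing triggers ChaseAI, which closes in, turns control rotation toward the target and spawns BP_BasicProjectile at the mesh transform.
; Falling out of bounds destroys the actor, while life and spawnpoint functions are stubs.
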(event OnSeePawn(PawnSensing)
  (params (Pawn :type Pawn%20Object%20Reference))
  ;[1 1 1] Observation script
  (Utilities|Casting|CastToBP_LinearAI Pawn)
  (CallFunction|ChaseAI Pawn))

(event Custom|Search%20Around
  ;[1 1 1] Search The Map
  (AI|AIMoveTo self (.RandomLocation (AI|Navigation|GetRandomReachablePointinRadius (Transformation|GetActorLocation) 2e+03 0 0)) 0 3e+02 false
    (:OnSuccess
      (Utilities|FlowControl|Delay 1.0))
    (:OnFail
      (if (AI|Components|NavMovement|IsFalling (Variables|Character|GetCharacterMovement)) :!label _label
        (Utilities|FlowControl|Delay 0.1)
        (goto _label)
        (else
          _))))
  (CallFunction|SearchAround))

(event Custom|Chase%20AI
  (params (TargetActor :type Actor%20Object%20Reference))
  ;[1 1 1] Chase entities
  (AI|AIMoveTo self "0, 0, 0" TargetActor 5e+02 false
    (:OnSuccess
      (CallFunction|Fire TargetActor))))

(event Custom|Fire
  (params (TargetActor :type Actor%20Object%20Reference))
  ;[1 1 1] Fire Projectile
  (Pawn|SetControlRotation (Pawn|GetController) (Math|Rotator|FindLookatRotation (Transformation|GetActorLocation) (Transformation|GetActorLocation TargetActor)))
  (Game|SpawnActorfromClass "/Game/FyreCracker/Weapons/Basic/BP_BasicProjectile.BP_BasicProjectile_C" (Transformation|GetWorldTransform (Variables|Character|GetMesh)) "Undefined" "MultiplyWithRoot" 0 4e+03 0))

(event Custom|BeginControllingCharacter
  ;[1 1 1] Begin Testing
  (if (AI|Components|NavMovement|IsFalling (Variables|Character|GetCharacterMovement)) :!label _label
    (Utilities|FlowControl|Delay 0.5)
    (goto _label)
    (else
      (CallFunction|SearchAround))))

(event EventBeginPlay
  ;[1 1 1] Initialize
  (AddComponent|AddACCharacter))

(fn ConstructionScript)

(fn AIFallsOutOfBounds
  (Actor|DestroyActor))

(fn GetLives
  (return 0))

(fn GetSpawnpoint
  (return ""))

(fn LoseLife
  (return false))