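; BP_CameraActor is a free-flying camera pawn that can shoot projectiles and reset to its starting point.
; On BeginPlay it enables input, stores its transform and follows controller rotation on all axes.
; Left and right Shift raise or lower FloatingPawnMovement max speed in steps, and R teleports back to the stored transform.
; Left click spawns BP_BasicProjectile from the mesh's transform, while T is only an AI-spawn placeholder that prints text.
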(event EventBeginPlay
  ;[1 1 1] Initialize
  (Input|EnableInput (Game|GetPlayerController 0))
  (Variables|Default|SetSpawnpoint (Transformation|GetActorTransform))
  (Variables|Default|SetbUseControllerRotationPitch true)
  (Variables|Default|SetbUseControllerRotationRoll true)
  (Variables|Default|SetbUseControllerRotationYaw true))

(event Input|KeyboardEvents|R
  (params (Key :type Key%20Structure :default "None"))
  ;[1 1 1] Respawn
  (:Pressed
    (Transformation|SetActorTransform (Variables|Default|GetSpawnpoint) false true)))

(event Input|KeyboardEvents|T
  (params (Key :type Key%20Structure :default "None"))
  ;[1 1 1] Spawn AI
  (:Pressed
    (Development|PrintString "Nothing yet...")))

(event Input|KeyboardEvents|LeftShift
  (params (Key :type Key%20Structure :default "None"))
  ;[1 1 1] Increase Flying Speed
  (:Pressed
    (bind _asfloating_pawn_movement (Utilities|Casting|CastToFloatingPawnMovement (Variables|Default|GetMovementComponent)))
    (Variables|/Script/Engine.FloatingPawnMovement|SetMaxSpeed _asfloating_pawn_movement (+ (Variables|Default|GetSpeed) (Variables|Default|GetDeltaSeed)))
    (Variables|Default|SetSpeed (+ (Variables|Default|GetSpeed) (Variables|Default|GetDeltaSeed)))))

(event Input|KeyboardEvents|RightShift
  (params (Key :type Key%20Structure :default "None"))
  ;[1 1 1] Decrease Flying Speed
  (:Pressed
    (bind _asfloating_pawn_movement (Utilities|Casting|CastToFloatingPawnMovement (Variables|Default|GetMovementComponent)))
    (Variables|/Script/Engine.FloatingPawnMovement|SetMaxSpeed _asfloating_pawn_movement (- (Variables|Default|GetSpeed) (Variables|Default|GetDeltaSeed)))
    (Variables|Default|SetSpeed (- (Variables|Default|GetSpeed) (Variables|Default|GetDeltaSeed)))))

(event Input|MouseEvents|LeftMouseButton
  (params (Key :type Key%20Structure :default "None"))
  (bind _meshcomponent (Variables|GetMeshComponent))
  (bind _returnvalue (Transformation|GetWorldTransform _meshcomponent))
  ;[1 1 1] Fire Projectile
  (:Pressed
    (Game|SpawnActorfromClass "/Game/FyreCracker/Weapons/Basic/BP_BasicProjectile.BP_BasicProjectile_C" (Math|Transform|MakeTransform (.location _returnvalue) (.rotation _returnvalue) "1.000000,1.000000,1.000000") "Undefined" "MultiplyWithRoot" 0 4e+03 0)))

(fn ConstructionScript)