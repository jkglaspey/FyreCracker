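; BP_BasicProjectile is a weapon projectile that explodes and destroys voxel terrain on impact.
; When its Sphere is hit, it adds an ACDestroyVoxel component, passes it the hit and destroys a randomly sized voxel sphere with block entities.
; It then spawns ExplosionActor, which is settable via SetExplosionActor, at the sphere's location and destroys itself.
; An unconnected DestroyVoxelSphere variant, noted as spawning no cubes, never runs.
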(event OnComponentHit(Sphere)
  (params (HitComponent :type Primitive%20Component%20Object%20Reference) (OtherActor :type Actor%20Object%20Reference) (OtherComp :type Primitive%20Component%20Object%20Reference) (NormalImpulse :type Vector :default "0, 0, 0") (Hit :type Hit%20Result%20Structure%20%28by%20ref%29))
  ;[1 1 1] Projectile hits voxel world
  (bind _returnvalue (AddComponent|AddACDestroyVoxel))
  (Default|SetCollisionHitResult _returnvalue Hit)
  (Default|DestroyVoxelSpherewithBlockEntities _returnvalue (Math|Random|RandomFloatinRange (Variables|Default|GetminimumExplosionSize) (Variables|Default|GetmaximumExplosionSize)))
  (Game|SpawnActorfromClass (Variables|Default|GetExplosionActor) (Math|Transform|MakeTransform (Transformation|GetWorldLocation (Variables|Default|GetSphere))) "Undefined" "MultiplyWithRoot" 0 0)
  (Actor|DestroyActor))

(fn ConstructionScript)

(fn SetExplosionActor
  (params (ExplosionActor :type Actor%20Class%20Reference))
  (Variables|Default|SetExplosionActor ExplosionActor))