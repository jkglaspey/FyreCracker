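; AI weapon projectile that blasts a spherical hole in voxel terrain when it hits something.
; On sphere hit, it adds an ACDestroyVoxel component at runtime, passes it the hit result, carves by ExplosionSize, spawns RFA_BasicExplosion and destroys itself.
; The construction script sets both initial and max projectile speed from LaunchSpeed.
; The destruction variant that spawns block entities is left unwired, so impacts produce no cubes.
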(event OnComponentHit(Sphere)
  (params (HitComponent :type Primitive%20Component%20Object%20Reference) (OtherActor :type Actor%20Object%20Reference) (OtherComp :type Primitive%20Component%20Object%20Reference) (NormalImpulse :type Vector :default "0, 0, 0") (Hit :type Hit%20Result%20Structure%20%28by%20ref%29))
  ;[1 1 1] Projectile hits voxel world
  (bind _returnvalue (AddComponent|AddACDestroyVoxel))
  (Default|SetCollisionHitResult _returnvalue Hit)
  ;[1 1 1] No cubes are spawned on collision
  (Default|DestroyVoxelSphere _returnvalue (Variables|Default|GetExplosionSize))
  (Game|SpawnActorfromClass "/Game/FyreCracker/Weapons/Basic/RFA_BasicExplosion.RFA_BasicExplosion_C" (Math|Transform|MakeTransform (Transformation|GetWorldLocation (Variables|Collision|GetSphere))) "Undefined" "MultiplyWithRoot" 0 0)
  (Actor|DestroyActor))

(fn ConstructionScript
  (bind _projectilemovement (Variables|Default|GetProjectileMovement))
  (bind _output_get (Variables|/Script/Engine.ProjectileMovementComponent|SetInitialSpeed _projectilemovement (Variables|Default|GetLaunchSpeed)))
  (Variables|/Script/Engine.ProjectileMovementComponent|SetMaxSpeed _projectilemovement _output_get))