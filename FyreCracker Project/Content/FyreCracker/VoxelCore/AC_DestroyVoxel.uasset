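; Actor component that carves explosion spheres out of the level's VoxelWorld at a stored hit impact point.
; DestroyVoxelSphere only removes the sphere.
; The block-entity variant first scatters short-lived physics cubes through filled voxels, scaling their count with explosion size and copying voxel colors via dynamic materials.
; It then removes the sphere and applies voxel physics, giving resulting cubes the same lifespan and ignored collision channels.
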(event Custom|DestroyVoxelSphereWithBlockEntities
  (params (explosionSize :type Float%20%28double-precision%29))
  (bind _singletonvoxelworld (Variables|Default|GetSingletonVoxelWorld))
  (bind _collisionhitresult (Variables|Default|GetCollisionHitResult))
  (bind _impactpoint (Collision|BreakHitResult _collisionhitresult))
  ;[1 1 1] Voxel Sphere Collision (With Blocks)
  ;;[0 0 0] Remove Initial Sphere
  (Variables|Default|SetexplosionSize explosionSize)
  (Utilities|FlowControl|Sequence
    (:then_0
      ;;[0 0 0] Spawn some cubes inside the removed sphere
      (for _index (range 0 (Math|Float|Truncate (* (Variables|Default|GetexplosionSize) (Variables|Default|GetBoxEntityCountScaling))))
        ;;;[1 1 1] Need to cache the result
        ;;; else random will be different
        (bind _output_get (Variables|Default|SetRandomPosition (+ _impactpoint (* (Math|Random|RandomUnitVector) (* (Variables|Default|GetexplosionSize) (Math|Float|Power (Math|Random|RandomFloat) 0.333333))))))
        ;;;[1 1 1] Check if the voxel is full
        (bind _value (Class|VoxelDataTools|GetValue _singletonvoxelworld (Class|VoxelWorld|GlobaltoLocal _singletonvoxelworld _output_get)))
        (if (<= _value 0.0)
          (bind _returnvalue (Game|SpawnActorfromClass "/Script/Engine.StaticMeshActor" (Math|Transform|MakeTransform (Variables|Default|GetRandomPosition) "0, 0, 0" (* (Math|Conversions|ToVector(Float) (/ (Variables|/Script/Voxel.VoxelWorld|GetVoxelSize _singletonvoxelworld) 1e+02)) (Variables|Default|GetBoxEntitySizeScaling))) "Undefined" "MultiplyWithRoot" 0 0))
          (Transformation|SetMobility _returnvalue "Movable")
          (Actor|SetLifeSpan _returnvalue (Variables|Default|GetblockLifeSpan))
          (Components|StaticMesh|SetStaticMesh (Variables|/Script/Engine.StaticMeshActor|GetStaticMeshComponent _returnvalue) "/Engine/BasicShapes/Cube.Cube")
          (Physics|SetSimulatePhysics (Variables|/Script/Engine.StaticMeshActor|GetStaticMeshComponent _returnvalue) true)
          (Collision|SetCollisionResponsetoChannel (Variables|/Script/Engine.StaticMeshActor|GetStaticMeshComponent _returnvalue) "ECC_Pawn" "ECR_Ignore")
          (Collision|SetCollisionResponsetoChannel (Variables|/Script/Engine.StaticMeshActor|GetStaticMeshComponent _returnvalue) "ECC_Visibility" "ECR_Ignore")
          (Collision|SetCollisionResponsetoChannel (Variables|/Script/Engine.StaticMeshActor|GetStaticMeshComponent _returnvalue) "ECC_GameTraceChannel1" "ECR_Ignore")
          (bind _material (Class|VoxelDataTools|GetMaterial _singletonvoxelworld (Class|VoxelWorld|GlobaltoLocal _singletonvoxelworld _output_get)))
          (bind _returnvalue_2 (Rendering|Material|CreateDynamicMaterialInstance "/Voxel/Examples/Materials/RGB/M_VoxelMaterial_Colors_Parameter.M_VoxelMaterial_Colors_Parameter" "None" "None" :!class /Script/Engine.KismetMaterialLibrary))
          (Rendering|Material|SetVectorParameterValue _returnvalue_2 "VertexColor" (Class|VoxelBlueprintLibrary|GetColor _material) :!class /Script/Engine.MaterialInstanceDynamic)
          (Rendering|Material|SetMaterial (Variables|/Script/Engine.StaticMeshActor|GetStaticMeshComponent _returnvalue) 0 _returnvalue_2)
          (Development|PrintString (Utilities|String|ToString(Integer) (Class|VoxelBlueprintLibrary|GetColor _material))))))
    (:then_1
      (Class|VoxelSphereTools|RemoveSphere _singletonvoxelworld _impactpoint (Variables|Default|GetexplosionSize))
      ;;[0 0 0] Voxel physics
      (bind _results (Class|VoxelPhysicsTools|ApplyVoxelPhysics _singletonvoxelworld (Class|VoxelBlueprintLibrary|MakeIntBoxfromGlobalPositionandRadius _singletonvoxelworld _impactpoint (Variables|Default|GetIntBoxRadius)) (Variables|Default|GetPartSpawner)))
      (for _array_element _results
        (bind _asvoxel_physics_part_spawner_result_cubes (Utilities|Casting|CastToVoxelPhysicsPartSpawnerResult_Cubes _array_element))
        (for _array_element_2 (Variables|/Script/Voxel.VoxelPhysicsPartSpawnerResult_Cubes|GetCubes _asvoxel_physics_part_spawner_result_cubes)
          (Actor|SetLifeSpan _array_element_2 (Variables|Default|GetblockLifeSpan))
          (Collision|SetCollisionResponsetoChannel (Variables|/Script/Engine.StaticMeshActor|GetStaticMeshComponent _array_element_2) "ECC_Pawn" "ECR_Ignore")
          (Collision|SetCollisionResponsetoChannel (Variables|/Script/Engine.StaticMeshActor|GetStaticMeshComponent _array_element_2) "ECC_Visibility" "ECR_Ignore")
          (Collision|SetCollisionResponsetoChannel (Variables|/Script/Engine.StaticMeshActor|GetStaticMeshComponent _array_element_2) "ECC_GameTraceChannel1" "ECR_Ignore"))))))

(event Custom|DestroyVoxelSphere
  (params (explosionSize :type Float%20%28double-precision%29))
  ;[1 1 1] Voxel Sphere Collision
  (Variables|Default|SetexplosionSize explosionSize)
  (Class|VoxelSphereTools|RemoveSphere (Variables|Default|GetSingletonVoxelWorld) (.ImpactPoint (Collision|BreakHitResult (Variables|Default|GetCollisionHitResult))) (Variables|Default|GetexplosionSize)))

(event EventBeginPlay
  ;[1 1 1] Initialize
  (bind _returnvalue (Actor|GetActorOfClass "/Script/Voxel.VoxelWorld"))
  (Variables|Default|SetSingletonVoxelWorld _returnvalue))

(fn SetCollisionHitResult
  (params (CollisionHitResult :type Hit%20Result%20Structure))
  (Variables|Default|SetCollisionHitResult CollisionHitResult))