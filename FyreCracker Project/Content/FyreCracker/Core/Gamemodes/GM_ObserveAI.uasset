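; GM_ObserveAI is a game mode for observing AI, though its BeginPlay is empty and its spawning logic is unwired, so it never runs.
; That disconnected logic reads NumAI from GI_Fyrecracker and spawns that many BP_LinearAI actors at the camera transform of the level's BP_FreeCamera.
; The construction script is empty.
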(event EventBeginPlay)

(fn ConstructionScript)